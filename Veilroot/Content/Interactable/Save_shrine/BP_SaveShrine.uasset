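; BP_SaveShrine is an interactable save shrine that triggers the player character's shrine interaction.
; Overlap events track whether an actor is inside and store the last one to enter.
; Tick polls that state with a HitSaveButton flag, which this graph only clears.
; When both are true, it casts the stored actor to BP_ThirdPersonCharacter, passes the CollisionBox world location to SaveShrineInteraction, and resets the flag.
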(event Collision|EventActorBeginOverlap
  (params (OtherActor :type Actor%20Object%20Reference))
  (Variables|Default|SetOverlaps? true)
  (Variables|Default|SetOther%20Actor OtherActor))

(event Collision|EventActorEndOverlap
  (params (OtherActor :type Actor%20Object%20Reference))
  (Variables|Default|SetOverlaps? false))

(event EventTick
  (params (DeltaSeconds :type Float%20%28single-precision%29))
  (if (and (Variables|Default|GetOverlaps?) (Variables|Default|GetHit_Save_Button?))
    (bind _asbp_third_person_character (Utilities|Casting|CastToBP_ThirdPersonCharacter (Variables|Default|GetOther%20Actor)))
    (Default|SaveShrineInteraction _asbp_third_person_character (Transformation|GetWorldLocation (Variables|Default|GetCollision%20box)))
    (Variables|Default|SetHit_Save_Button? false)))

(fn ConstructionScript)
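; BP_Groove_Enemy is a non-boss enemy that spots the player and tracks its own health.
; PawnSensing sightings raise SeeEnemy, which a 0.2-second retriggerable delay clears while resetting SeenTarget's DoOnce gate.
; SeenTarget sets the AI blackboard's hasSeenPlayer for the player character, rechecking every second until sight is lost, then clears it.
; Damage reduces Health, but death is only a debug print so far.
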(event OnSeePawn(PawnSensing)
  (params (Pawn :type Pawn%20Object%20Reference))
  (Variables|Default|SetIsEnemy Pawn)
  (Variables|Default|SetseeEnemy true)
  (Utilities|FlowControl|Sequence
    (:then_0
      (CallFunction|SeenTarget Pawn))
    (:then_1
      (Utilities|FlowControl|RetriggerableDelay 0.2)
      (Variables|Default|SetseeEnemy false)
      (CallFunction|ResetSence))))

(event Custom|SeenTarget
  (params (PawnObjReference :type Pawn%20Object%20Reference))
  (Utilities|FlowControl|DoOnce false
    (:Completed
      (Utilities|Casting|CastToBP_ThirdPersonCharacter PawnObjReference :!label _label)
      (AI|Components|Blackboard|SetValueasBool (AI|GetBlackboard (AI|GetAIController self)) (Utilities|Name|MakeLiteralName "hasSeenPlayer") true)
      (Utilities|FlowControl|Delay 1.0)
      (if (Variables|Default|GetseeEnemy)
        (goto _label)
        (else
          (Utilities|Casting|CastToBP_ThirdPersonCharacter PawnObjReference)
          (AI|Components|Blackboard|SetValueasBool (AI|GetBlackboard (AI|GetAIController self)) (Utilities|Name|MakeLiteralName "hasSeenPlayer") false))))))

(event Custom|ResetSence
  (Utilities|FlowControl|DoOnce false) ; enters at Reset
)

(event EventBeginPlay)

(event Collision|EventActorBeginOverlap
  (params (OtherActor :type Actor%20Object%20Reference)))

(event Game|Damage|EventAnyDamage
  (params (Damage :type Float%20%28single-precision%29) (DamageType :type Damage%20Type%20Object%20Reference) (InstigatedBy :type Controller%20Object%20Reference) (DamageCauser :type Actor%20Object%20Reference))
  (Variables|Default|SetHealth (- (Variables|Default|GetHealth) Damage))
  (if (<= (Variables|Default|GetHealth) 0.0)
    ;[0.15 0.15 0.15 0.5] Pak nahradit funkcema
    (Development|PrintString "Died")
    (else
      (Development|PrintString (Utilities|String|ToString(Float) (Variables|Default|GetHealth))))))

(fn ConstructionScript)